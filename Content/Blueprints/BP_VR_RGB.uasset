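; VR Blueprint that shows a RealSense RGB camera feed on a plane, using a floor-level tracking origin.
; On BeginPlay it creates a dynamic M_Video material, places the image plane at a configurable distance and scales it from that distance and the camera's field of view.
; Each tick, when RealsenseRGB receives a frame, it assigns the camera texture to the material's VideoTexture parameter.
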(event EventBeginPlay
  (bind _imageplane (Variables|Default|GetImagePlane))
  (bind _relativelocation (Variables|/Script/Engine.SceneComponent|GetRelativeLocation _imageplane))
  (bind (_x _y _z) (Math|Vector|BreakVector _relativelocation))
  (Class|HeadMountedDisplayFunctionLibrary|SetTrackingOrigin "Floor")
  ;[1 1 1] Get realsense textures
  (bind _returnvalue (Class|RealsenseRGBComponent|GetTextureRGB (Variables|Default|GetRealsenseRGB)))
  (Variables|Default|SetT_RGB _returnvalue)
  ;[1 1 1] create dynamic materials
  (bind _returnvalue_2 (Rendering|Material|CreateDynamicMaterialInstance (Variables|Default|GetPlaneRGB) 0 "/RealSensePlugin/Materials/M_Video.M_Video" "None" :!class /Script/Engine.PrimitiveComponent))
  (Variables|Default|SetM_RGB_dyn _returnvalue_2)
  ;[1 1 1] Transform image plane
  (Transformation|SetRelativeLocation _imageplane (Math|Vector|MakeVector (Variables|Default|GetImagePlaneDistance) _y _z) false false)
  (CallFunction|SetPlaneScale (Variables|Default|GetPlaneRGB)))

(event EventTick
  (params (DeltaSeconds :type Float%20%28single-precision%29))
  ;[1 1 1] Udpate Textures
  (bind _returnvalue (Class|RealsenseRGBComponent|ReceiveFrame (Variables|Default|GetRealsenseRGB)))
  (if _returnvalue
    (Rendering|Material|SetTextureParameterValue (Variables|Default|GetM_RGB_dyn) "VideoTexture" (Variables|Default|GetT_RGB))))

(fn ConstructionScript)

(fn SetPlaneScale
  (params (Plane :type Static%20Mesh%20Component%20Object%20Reference))
  (bind _imageplanedistance (Variables|Default|GetImagePlaneDistance))
  (bind _realsensergb (Variables|Default|GetRealsenseRGB))
  (bind _returnvalue (/ _imageplanedistance 1e+02))
  (bind _horizontalfov (Variables|/Script/RealSensePlugin.RealsenseRGBComponent|GetHorizontalFOV _realsensergb))
  (bind _returnvalue_2 (Math|Trig|Tan(Degrees) _horizontalfov))
  (bind _returnvalue_3 (* _returnvalue _returnvalue_2))
  (Transformation|SetRelativeScale3D Plane (Math|Vector|MakeVector (* (/ (Variables|/Script/RealSensePlugin.RealsenseRGBComponent|GetVerticalFOV _realsensergb) _horizontalfov) _returnvalue_3) _returnvalue_3 (.Z (Math|Vector|BreakVector (Variables|/Script/Engine.SceneComponent|GetRelativeScale3D Plane))))))