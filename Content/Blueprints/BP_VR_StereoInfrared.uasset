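; VR Blueprint that shows a RealSense stereo infrared camera feed on separate left and right eye planes.
; BeginPlay sets a floor tracking origin, caches both textures from the RealsenseInfraredStereo component and creates a dynamic material for each plane.
; BeginPlay and every Tick then call UpdateTextures and, on success, assign the textures to the Left_Eye and Right_Eye material parameters.
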(event EventBeginPlay
  (bind _realsenseinfraredstereo (Variables|Default|GetRealsenseInfraredStereo))
  (Class|HeadMountedDisplayFunctionLibrary|SetTrackingOrigin "Floor")
  ;[1 1 1] Get realsense textures
  (bind _returnvalue (Class|RealsenseInfraredStereoComponent|GetTextureLeft _realsenseinfraredstereo))
  (Variables|Default|SetT_Left _returnvalue)
  (bind _returnvalue_2 (Class|RealsenseInfraredStereoComponent|GetTextureRight _realsenseinfraredstereo))
  (Variables|Default|SetT_Right _returnvalue_2)
  ;[1 1 1] create dynamic materials
  (bind _returnvalue_3 (Rendering|Material|CreateDynamicMaterialInstance (Variables|Default|GetPlaneLeft) 0 "/RealSensePlugin/Materials/M_VideoInfraredLeft.M_VideoInfraredLeft" "None" :!class /Script/Engine.PrimitiveComponent))
  (Variables|Default|SetM_Left_dyn _returnvalue_3)
  (bind _returnvalue_4 (Rendering|Material|CreateDynamicMaterialInstance (Variables|Default|GetPlaneRight) 0 "/RealSensePlugin/Materials/M_VideoInfraredRight.M_VideoInfraredRight" "None" :!class /Script/Engine.PrimitiveComponent))
  (Variables|Default|SetM_Right_dyn _returnvalue_4)
  ;[1 1 1] Udpate Textures
  (bind _returnvalue_5 (Class|RealsenseInfraredStereoComponent|UpdateTextures (Variables|Default|GetRealsenseInfraredStereo)))
  (if _returnvalue_5
    (Rendering|Material|SetTextureParameterValue (Variables|Default|GetM_Left_dyn) "Left_Eye" (Variables|Default|GetT_Left))
    (Rendering|Material|SetTextureParameterValue (Variables|Default|GetM_Right_dyn) "Right_Eye" (Variables|Default|GetT_Right))))

(event EventTick
  (params (DeltaSeconds :type Float%20%28single-precision%29))
  ;[1 1 1] Udpate Textures
  (bind _returnvalue (Class|RealsenseInfraredStereoComponent|UpdateTextures (Variables|Default|GetRealsenseInfraredStereo)))
  (if _returnvalue
    (Rendering|Material|SetTextureParameterValue (Variables|Default|GetM_Left_dyn) "Left_Eye" (Variables|Default|GetT_Left))
    (Rendering|Material|SetTextureParameterValue (Variables|Default|GetM_Right_dyn) "Right_Eye" (Variables|Default|GetT_Right))))

(fn ConstructionScript)