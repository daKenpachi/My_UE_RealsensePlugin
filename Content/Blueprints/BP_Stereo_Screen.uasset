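; BP_Stereo_Screen is an actor that displays left and right infrared video textures on two image planes.
; On BeginPlay it creates a dynamic M_VideoInfrared material for each plane and sets each plane's horizontal scale from its width-to-height ratio.
; Each Tick it calls UpdateTextures, which is not defined in this graph, and on success pushes both textures into the materials' VideoTexture parameter.
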(event EventBeginPlay
  (bind _infraredright (Variables|Default|GetInfraredRight))
  (bind _infraredleft (Variables|Default|GetInfraredLeft))
  ;[1 1 1] Create Dynamic Materials for planes
  (bind _returnvalue (Rendering|Material|CreateDynamicMaterialInstance _infraredleft 0 "/RealSensePlugin/Materials/M_VideoInfrared.M_VideoInfrared" "None" :!class /Script/Engine.PrimitiveComponent))
  (bind _output_get (Variables|Default|SetM_Left_dyn _returnvalue))
  (Rendering|Material|SetMaterial _infraredleft 0 _output_get)
  (bind _returnvalue_2 (Rendering|Material|CreateDynamicMaterialInstance _infraredright 0 "/RealSensePlugin/Materials/M_VideoInfrared.M_VideoInfrared" "None" :!class /Script/Engine.PrimitiveComponent))
  (bind _output_get_2 (Variables|Default|SetM_Right_dny _returnvalue_2))
  (Rendering|Material|SetMaterial _infraredright 0 _output_get_2)
  ;[1 1 1] Set correct image plane scales
  (Transformation|SetRelativeScale3D (Variables|Default|GetInfraredLeft) (Math|Vector|MakeVector (/ (Math|Conversions|ToFloat(Integer) (Variables|Default|GetWidthLeft)) (Math|Conversions|ToFloat(Integer) (Variables|Default|GetHeightLeft))) 1.0 1.0))
  (Transformation|SetRelativeScale3D (Variables|Default|GetInfraredRight) (Math|Vector|MakeVector (/ (Math|Conversions|ToFloat(Integer) (Variables|Default|GetWidthRight)) (Math|Conversions|ToFloat(Integer) (Variables|Default|GetHeightRight))) 1.0 1.0)))

(event Collision|EventActorBeginOverlap
  (params (OtherActor :type Actor%20Object%20Reference)))

(event EventTick
  (params (DeltaSeconds :type Float%20%28single-precision%29))
  (bind _returnvalue (Class|RealsenseInfraredStereoCamera|UpdateTextures))
  (if _returnvalue
    (Rendering|Material|SetTextureParameterValue (Variables|Default|GetM_Left_dyn) "VideoTexture" (Variables|Default|GetTextureLeft))
    (Rendering|Material|SetTextureParameterValue (Variables|Default|GetM_Right_dny) "VideoTexture" (Variables|Default|GetTextureRight))))

(fn ConstructionScript)