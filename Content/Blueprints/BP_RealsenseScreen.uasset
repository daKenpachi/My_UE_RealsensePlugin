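; BP_RealsenseScreen is an actor that displays live color and depth frames, apparently from a RealSense camera, on two planes.
; BeginPlay creates a dynamic instance of M_Video for VideoPlane and another for DepthPlane.
; Each Tick calls ReceiveFrames, then pushes TextureFromVideo and TextureFromDepth into the respective material's video texture parameter.
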(event EventBeginPlay
  (bind _videoplane (Variables|Default|GetVideoPlane))
  (bind _depthplane (Variables|Default|GetDepthPlane))
  ;[1 1 1] Create Dynamic Materials for planes
  (bind _returnvalue (Rendering|Material|CreateDynamicMaterialInstance _videoplane 0 "/RealSensePlugin/Materials/M_Video.M_Video" "None" :!class /Script/Engine.PrimitiveComponent))
  (bind _output_get (Variables|Default|SetM_Color_dyn _returnvalue))
  (Rendering|Material|SetMaterial _videoplane 0 _output_get)
  (bind _returnvalue_2 (Rendering|Material|CreateDynamicMaterialInstance _depthplane 0 "/RealSensePlugin/Materials/M_Video.M_Video" "None" :!class /Script/Engine.PrimitiveComponent))
  (bind _output_get_2 (Variables|Default|SetM_Depth_dyn _returnvalue_2))
  (Rendering|Material|SetMaterial _depthplane 0 _output_get_2))

(event EventTick
  (params (DeltaSeconds :type Float%20%28single-precision%29))
  ;[1 1 1] Update Textures with new frames
  (Class|RealSenseComponent|ReceiveFrames)
  (Rendering|Material|SetTextureParameterValue (Variables|Default|GetM_Color_dyn) "VideoTexture" (Variables|Default|GetTextureFromVideo))
  (Rendering|Material|SetTextureParameterValue (Variables|Default|GetM_Depth_dyn) "VIdeoTexture" (Variables|Default|GetTextureFromDepth)))

(fn ConstructionScript)