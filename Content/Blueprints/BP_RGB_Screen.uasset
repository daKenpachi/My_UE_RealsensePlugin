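; RGB screen Blueprint that displays received video frames on a plane mesh.
; On BeginPlay it creates a dynamic instance of M_Video for the plane and scales its X by the width-to-height ratio to correct the image proportions.
; Each Tick it calls ReceiveFrames and, on success, pushes TextureFromVideo into the material's VideoTexture parameter.
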(event EventBeginPlay
  (bind _planergb (Variables|Default|GetPlaneRGB))
  ;[1 1 1] Create Dynamic Material
  (bind _returnvalue (Rendering|Material|CreateDynamicMaterialInstance _planergb 0 "/RealSensePlugin/Materials/M_Video.M_Video" "None" :!class /Script/Engine.PrimitiveComponent))
  (bind _output_get (Variables|Default|SetM_RGB_dyn _returnvalue))
  (Rendering|Material|SetMaterial _planergb 0 _output_get)
  ;[1 1 1] Set correct image plane width
  (Transformation|SetRelativeScale3D (Variables|Default|GetPlaneRGB) (Math|Vector|MakeVector (/ (Math|Conversions|ToFloat(Integer) (Variables|Default|GetWidth_c)) (Math|Conversions|ToFloat(Integer) (Variables|Default|GetHeight_c))) 1.0 1.0)))

(event EventTick
  (params (DeltaSeconds :type Float%20%28single-precision%29))
  (bind _returnvalue (Class|RealSenseRGBCamera|ReceiveFrames))
  (if _returnvalue
    (Rendering|Material|SetTextureParameterValue (Variables|Default|GetM_RGB_dyn) "VideoTexture" (Variables|Default|GetTextureFromVideo))))

(fn ConstructionScript)